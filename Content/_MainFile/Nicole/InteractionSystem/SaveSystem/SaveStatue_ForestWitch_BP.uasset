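; Forest Witch save statue Blueprint that the player interacts with to open or close a save screen.
; Interact toggles the SaveScreen widget, passing it a reference to the statue and switching cursor visibility and input mode to match.
; When the screen opens, the statue also copies its SavePointLocation onto Player_BP.
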(event `/Game/_MainFile/Nicole/InteractionSystem/Interact_BPI.Interact`
  (bind _returnvalue (`GameplayStatics.GetPlayerController` 0))
  (bind _returnvalue_2 (`GameplayStatics.GetPlayerController` 0))
  (if (`self.SaveScreenOpen?`)
    (`Widget.RemoveFromParent` (`self.SaveScreenRef`))
    (set `PlayerController.bShowMouseCursor` false _returnvalue)
    (`WidgetBlueprintLibrary.SetInputMode_GameOnly` _returnvalue)
    (set `self.SaveScreenOpen?` false)
    (else
      (bind _returnvalue_3 (`|CreateWidget` "/Game/_MainFile/Nicole/InteractionSystem/SaveSystem/SaveScreen_w.SaveScreen_w_C"))
      (set `/Game/_MainFile/Nicole/InteractionSystem/SaveSystem/SaveScreen_w.ForsetWitchStatueRef` self _returnvalue_3)
      (bind _output_get (set `self.SaveScreenRef` _returnvalue_3))
      (`UserWidget.AddToViewport` _output_get 0)
      (set `PlayerController.bShowMouseCursor` true _returnvalue_2)
      (`WidgetBlueprintLibrary.SetInputMode_GameAndUIEx` _returnvalue_2 (`self.SaveScreenRef`))
      (set `self.SaveScreenOpen?` true)
      (bind _asplayer_bp (cast `/Game/ThirdPerson/Blueprints/Player_BP` (`GameplayStatics.GetPlayerCharacter` 0)))
      (set `/Game/ThirdPerson/Blueprints/Player_BP.SavePointLocation` (`self.SavePointLocation`) _asplayer_bp))))

(fn `UserConstructionScript`
  (`parent.UserConstructionScript`))