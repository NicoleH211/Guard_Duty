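; Shopkeeper Blueprint that toggles a shop UI when the player interacts with it.
; On opening, it looks up each expected inventory enum as a row name in the item info data table and adds found items uniquely to its inventory.
; It then creates the shop widget with itself as shopkeeper and switches to game-and-UI input with a cursor.
; Interacting again removes the widget and restores game-only input.
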(event `/Game/_MainFile/Nicole/InteractionSystem/Interact_BPI.Interact`
  (bind _returnvalue (`GameplayStatics.GetPlayerController` 0))
  (bind _inventoryexpected (`self.InventoryExpected`))
  (if (`self.Shop Open?`)
    (`Widget.RemoveFromParent` (`self.Shop Widget`))
    (`WidgetBlueprintLibrary.SetInputMode_GameOnly` _returnvalue)
    (set `PlayerController.bShowMouseCursor` false _returnvalue)
    (set `self.Shop Open?` false)
    (else
      (for _index (range (`KismetArrayLibrary.Array_Length` _inventoryexpected))
        (bind _returnvalue_2 (`|GetDataTableRow` "/Game/_MainFile/Nicole/InteractionSystem/ItemInfo_DT.ItemInfo_DT" (`KismetStringLibrary.Conv_StringToName` (`|GetEnumeratorNameAsString` (`|GetArrayItem` _inventoryexpected _index))))
          (:`then`
            (`KismetArrayLibrary.Array_AddUnique` (`self.Inventory`) _returnvalue_2))))
      (`self.Show Shop`))))

(event `Show Shop`
  (bind _returnvalue (`GameplayStatics.GetPlayerController` 0))
  (bind _returnvalue_2 (`|CreateWidget` "/Game/_MainFile/Nicole/InteractionSystem/ShopKeeper/Shop_W.Shop_W_C"))
  (set `/Game/_MainFile/Nicole/InteractionSystem/ShopKeeper/Shop_W.ShopKeeper` self _returnvalue_2)
  (bind _output_get (set `self.Shop Widget` _returnvalue_2))
  (`UserWidget.AddToViewport` _output_get 0)
  (`WidgetBlueprintLibrary.SetInputMode_GameAndUIEx` _returnvalue _output_get)
  (set `PlayerController.bShowMouseCursor` true _returnvalue)
  (set `self.Shop Open?` true))

(fn `UserConstructionScript`
  (`parent.UserConstructionScript`))