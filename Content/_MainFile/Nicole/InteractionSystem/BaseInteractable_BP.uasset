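; Base interactable actor for items that the player picks up.
; Its construction script converts the ItemName enum to a row name and copies the matching ItemInfo_DT row into ItemInfo.
; On Interact, it casts player character 0 to Player_BP, passes ItemInfo to PickupItem and destroys itself.
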(event `/Game/_MainFile/Nicole/InteractionSystem/Interact_BPI.Interact`
  (bind _asplayer_bp (cast `/Game/ThirdPerson/Blueprints/Player_BP` (`GameplayStatics.GetPlayerCharacter` 0)))
  (`/Game/ThirdPerson/Blueprints/Player_BP.Pickup Item` _asplayer_bp (`self.ItemInfo`))
  (`self.K2_DestroyActor`))

(fn `UserConstructionScript`
  (bind _returnvalue (`|GetDataTableRow` "/Game/_MainFile/Nicole/InteractionSystem/ItemInfo_DT.ItemInfo_DT" (`KismetStringLibrary.Conv_StringToName` (`|GetEnumeratorNameAsString` (`self.ItemName`))))
    (:`then`
      (set `self.ItemInfo` _returnvalue))))