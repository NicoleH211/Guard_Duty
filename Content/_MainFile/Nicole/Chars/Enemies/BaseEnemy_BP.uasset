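; BaseEnemy_BP is an enemy Blueprint that handles roaming behaviour, starting at BeginPlay.
; BehaviourUnit alternates two AIMoveTo modes: a random reachable point within RoamRadius, then the referenced patrol point, with random waits between moves.
; After each random roam, it scans all EnemyPatrolPoint_BP actors and switches to any closer one.
; The loop re-calls itself only after successful moves while not attacking the player, and stops when dead.
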(event `self.ReceiveBeginPlay`
  (`self.Behaviour Unit`))

(event `Behaviour Unit`
  (if (not (`self.Dead?`))
    (switch `/Game/_MainFile/Nicole/Chars/Enemies/BehaviourModes_E` (`self.Behaviour Mode`)
      (:`NewEnumerator0`
        (`|AIMoveTo` self (`NavigationSystemV1.K2_GetRandomReachablePointInRadius` (`self.K2_GetActorLocation`) (`self.Roam Radius`) null null) null
          (:`OnSuccess`
            (`self.Update Patrol Point`)
            (if (not (`self.Attacking Player?`))
              (`KismetSystemLibrary.Delay` (`KismetMathLibrary.RandomFloatInRange` (`self.Min Wait`) (`self.Max Wait`)))
              (set `self.Behaviour Mode` "NewEnumerator1")
              (`self.Behaviour Unit`)))))
      (:`NewEnumerator1`
        (`|AIMoveTo` self (0.0 0.0 0.0) (`self.Patrol Point Ref`)
          (:`OnSuccess`
            (if (not (`self.Attacking Player?`))
              (`KismetSystemLibrary.Delay` (`KismetMathLibrary.RandomFloatInRange` (`self.Min Wait`) (`self.Max Wait`)))
              (set `self.Behaviour Mode` "NewEnumerator0")
              (`self.Behaviour Unit`))))))))

(fn `Update Patrol Point`
  (bind _outactors (`GameplayStatics.GetAllActorsOfClass` "/Game/_MainFile/Nicole/Chars/Enemies/EnemyPatrolPoint_BP.EnemyPatrolPoint_BP_C"))
  (for _array_element _outactors
    (if (< (`self.GetDistanceTo` _array_element self) (`self.GetDistanceTo` (`self.Patrol Point Ref`) self))
      (set `self.Patrol Point Ref` _array_element))))

(fn `UserConstructionScript`)