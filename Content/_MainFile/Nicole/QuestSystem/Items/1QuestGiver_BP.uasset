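; Quest giver actor that shows a floating "!" or "?" marker and opens a quest screen on interact.
; On BeginPlay it filters its quest list by data table prerequisites and the player's completed quests.
; The marker switches to "?" when a listed quest is accepted, and hides when none remain.
; Interact toggles the widget, cursor and slowed time; closing it has every quest giver restore its saved list and recheck prerequisites.
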(event `/Game/_MainFile/Nicole/InteractionSystem/Interact_BPI.Interact`
  (bind _returnvalue (`GameplayStatics.GetPlayerController` 0))
  (bind _returnvalue_2 (`GameplayStatics.GetPlayerController` 0))
  (if (`self.QuestScreenOpen?`)
    (`Widget.RemoveFromParent` (`self.Quest Screen Ref`))
    (set `self.QuestScreenOpen?` false)
    (`WidgetBlueprintLibrary.SetInputMode_GameOnly` _returnvalue)
    (`GameplayStatics.SetGlobalTimeDilation` 1.0) ; Can set to 0 for freeze time
    (set `PlayerController.bShowMouseCursor` false _returnvalue)
    (bind _outactors (`GameplayStatics.GetAllActorsOfClass` "1QuestGiver_BP_C"))
    (for _ _outactors
      (`self.Recheck Prereqs`))
    (else
      (`/Engine/EditorBlueprintResources/StandardMacros.IsValid` (`self.Quest Screen Ref`)
        (:`Is Valid`
          _)
        (:`Is Not Valid`
          (bind _returnvalue_3 (`|CreateWidget` "/Game/_MainFile/Nicole/QuestSystem/Widgets/QuestScreen_W.QuestScreen_W_C" null self))
          (bind _output_get (set `self.Quest Screen Ref` _returnvalue_3))))
      (`UserWidget.AddToViewport` _output_get 0)
      (set `self.QuestScreenOpen?` true)
      (`WidgetBlueprintLibrary.SetInputMode_GameAndUIEx` _returnvalue_2 _output_get)
      (set `PlayerController.bShowMouseCursor` true _returnvalue_2)
      (`GameplayStatics.SetGlobalTimeDilation` 0.25) ; Can set to 0 for freeze time
    )))

(event `self.ReceiveBeginPlay`
  (bind _textrender (`self.TextRender`))
  (bind _quest_list (`self.Quest List`))
  (`|ExecutionSequence` :!label _label
    (:`then_0`
      (set `self.Saved Quests` _quest_list)
      (for _array_element _quest_list
        (bind _returnvalue (`|GetDataTableRow` "/Game/_MainFile/Nicole/QuestSystem/Quest1_DT.Quest1_DT" (`KismetStringLibrary.Conv_StringToName` (`|GetEnumeratorNameAsString` _array_element)))
          (:`then`
            (bind _asplayer_bp (cast `/Game/ThirdPerson/Blueprints/Player_BP` (`GameplayStatics.GetPlayerCharacter` 0)))
            (set `self.Player BP Ref` _asplayer_bp)
            (for _array_element_2 (`.PrereqNeeded_45_4D3AC27147984484778B379FF61BA241` (break `/Game/_MainFile/Nicole/QuestSystem/QuestInfo_S` _returnvalue))
              (if (not (`KismetArrayLibrary.Array_Contains` (`/Game/ThirdPerson/Blueprints/Player_BP.Completed Quests` _asplayer_bp) _array_element_2))
                (`KismetArrayLibrary.Array_RemoveItem` (`self.Quest List`) _array_element)))))))
    (:`then_1`
      (for _array_element_3 (`/Game/ThirdPerson/Blueprints/Player_BP.Completed Quests` (`self.Player BP Ref`))
        (if (`KismetArrayLibrary.Array_Contains` (`self.Quest List`) _array_element_3)
          (`KismetArrayLibrary.Array_RemoveItem` (`self.Quest List`) _array_element_3)
          (`KismetArrayLibrary.Array_RemoveItem` (`self.Saved Quests`) _array_element_3)
          (`KismetSystemLibrary.PrintString` "Quest Removed")))
      (if (> (`KismetArrayLibrary.Array_Length` (`self.Quest List`)) 0)
        (bind _output_get (set `self.Value` "!"))
        (`TextRenderComponent.K2_SetText` _textrender _output_get)
        (`SceneComponent.SetVisibility` _textrender true false)
        (`self.Compare`)
        (else
          (`SceneComponent.SetVisibility` _textrender false false))))))

(event `Recheck Prereqs`
  (set `self.Quest List` (`self.Saved Quests`))
  (goto _label))

(event `Compare`
  (for _array_element (`self.Quest List`)
    (if (`KismetArrayLibrary.Array_Contains` (`/Game/ThirdPerson/Blueprints/Player_BP.Accepted Quests` (`self.Player BP Ref`)) _array_element)
      (bind _output_get (set `self.Value` "?"))
      (`TextRenderComponent.K2_SetText` (`self.TextRender`) _output_get)
      (set `self.Found?` true)))
  (if (not (`self.Found?`))
    (bind _output_get_2 (set `self.Value` "!"))
    (`TextRenderComponent.K2_SetText` (`self.TextRender`) _output_get_2)))

(fn `UserConstructionScript`
  (`parent.UserConstructionScript`))