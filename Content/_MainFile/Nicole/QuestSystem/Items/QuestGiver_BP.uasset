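; Quest giver Blueprint that toggles a quest screen when the player interacts with it.
; On first open it creates a QuestScreen_W widget with itself passed as QuestGiver, then reuses that widget while it stays valid.
; Opening adds the screen to the viewport with Game and UI input, focus and mouse cursor.
; Closing removes it and restores game-only input with the cursor hidden.
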(event `/Game/_MainFile/Nicole/InteractionSystem/Interact_BPI.Interact`
  (bind _returnvalue (`GameplayStatics.GetPlayerController` 0))
  (bind _returnvalue_2 (`GameplayStatics.GetPlayerController` 0))
  (if (`self.QuestScreenOpen?`)
    (`Widget.RemoveFromParent` (`self.Quest Screen Ref`))
    (set `self.QuestScreenOpen?` false)
    (`WidgetBlueprintLibrary.SetInputMode_GameOnly` _returnvalue)
    (set `PlayerController.bShowMouseCursor` false _returnvalue)
    (else
      (`/Engine/EditorBlueprintResources/StandardMacros.IsValid` (`self.Quest Screen Ref`)
        (:`Is Valid`
          _)
        (:`Is Not Valid`
          (bind _returnvalue_3 (`|CreateWidget` "/Game/_MainFile/Nicole/QuestSystem/Widgets/QuestScreen_W.QuestScreen_W_C" null self))
          (bind _output_get (set `self.Quest Screen Ref` _returnvalue_3))))
      (`UserWidget.AddToViewport` _output_get 0)
      (set `self.QuestScreenOpen?` true)
      (`WidgetBlueprintLibrary.SetInputMode_GameAndUIEx` _returnvalue_2 _output_get)
      (set `PlayerController.bShowMouseCursor` true _returnvalue_2))))

(fn `UserConstructionScript`
  (`parent.UserConstructionScript`))